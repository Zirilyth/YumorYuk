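; CookingPot is an actor that collects ingredients dropped into it.
; On sphere overlap, it writes the actor's first tag into the first empty of two ingredient slots on the GiantController.
; It then destroys the actor and calls Oncook on the game mode's Hud.
; When both slots are full, the actor is still destroyed and Oncook still fires, but its tag is not stored.
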(event OnComponentBeginOverlap(Sphere)
  (params (OverlappedComponent :type Primitive%20Component%20Object%20Reference) (OtherActor :type Actor%20Object%20Reference) (OtherComp :type Primitive%20Component%20Object%20Reference) (OtherBodyIndex :type Integer) (bFromSweep :type Boolean) (SweepResult :type Hit%20Result%20Structure%20%28by%20ref%29))
  (bind _tags (Variables|/Script/Engine.Actor|GetTags OtherActor))
  (bind _output (Utilities|Array|Get(acopy) _tags))
  (bind _returnvalue (Utilities|String|ToString(Name) _output))
  (bind _asgiant_controller (Utilities|Casting|CastToGiantController (Game|GetPlayerController 0)))
  (Development|PrintString (Utilities|String|ToString(Name) _output))
  (if (Utilities|Enum|Equal(Enum) (stale _output_get) "")
    (bind _output_get (Variables|/Game/YumOrYuk/Blueprints/Giant/GiantController.GiantController_C|SetIngredient1 _asgiant_controller _returnvalue))
    (elif (Utilities|Enum|Equal(Enum) (stale _output_get_2) "")
      (bind _output_get_2 (Variables|/Game/YumOrYuk/Blueprints/Giant/GiantController.GiantController_C|SetIngredient2 _asgiant_controller _returnvalue))
      (else
        (Utilities|Casting|CastToYumorYukGameMode (Game|GetGameMode)))))
  (Actor|DestroyActor OtherActor)
  (bind _asyumor_yuk_game_mode (Utilities|Casting|CastToYumorYukGameMode (Game|GetGameMode)))
  (Default|Oncook (Variables|/Game/YumOrYuk/Blueprints/YumorYukGameMode.YumorYukGameMode_C|GetHud _asyumor_yuk_game_mode)))

(fn ConstructionScript)